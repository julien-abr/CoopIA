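; BP_Canon is an automatic cannon that fires BP_Bullet projectiles at a fixed interval.
; On BeginPlay it starts a looping timer set by CanonCooldown, which calls Shoot.
; Each shot spawns a bullet at the FirePoint transform, plays cannon and projectile sounds at the actor's location, and spawns a scaled-up Niagara water-hit effect at the VFX component.
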(event Custom|Shoot
  (bind _firepoint (Variables|Default|GetFirePoint))
  (bind _vfx (Variables|Default|GetVFX))
  (bind _returnvalue (Transformation|GetWorldTransform _firepoint))
  (bind _returnvalue_2 (Transformation|GetWorldTransform _vfx))
  (Utilities|FlowControl|Sequence
    (:then_0
      ;[0.7627 1 0.7531] SD
      (Audio|PlaySoundatLocation "/Game/Sound/SD/Canon/CanonCue.CanonCue" (Transformation|GetActorLocation) "0, 0, 0" 1.0 1.0 0.0 0 0 0 0)
      (Game|SpawnActorfromClass "/Game/CoopIA/Blueprints/Ingredient/Canon/BP_Bullet.BP_Bullet_C" (Math|Transform|MakeTransform (.location _returnvalue) (.rotation _returnvalue) "1.000000,1.000000,1.000000") "Undefined" "MultiplyWithRoot" 0 0)
      ;[0.7627 1 0.7531] SD
      (Audio|PlaySoundatLocation "/Game/Sound/SD/Canon/Projectiles/ProjectilesCue.ProjectilesCue" (Transformation|GetActorLocation) "0, 0, 0" 1.0 1.0 0.0 0 0 0 0))
    (:then_1
      (Niagara|SpawnSystematLocation "/Game/Axelle/FX/NS_Water_Hit.NS_Water_Hit" (.location _returnvalue_2) (.rotation _returnvalue_2) "4.500000,4.500000,4.500000"))))

(event EventBeginPlay
  (Utilities|Time|SetTimerbyEvent (delegate Custom|Shoot) (Variables|Default|GetCanonCooldown) true))

(fn ConstructionScript)