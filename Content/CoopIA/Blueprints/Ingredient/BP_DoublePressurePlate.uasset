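; Double pressure plate Blueprint that gives audio and visual feedback when pressed and released.
; OnPressure plays a sound and switches both plate bodies to the activated material; OnEndPressure restores the default material.
; Each press also restarts PressurePlateEffect from its relative origin, moving it by the offset between the referenced Object and the pressure position, then deactivating it when the move completes.
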(event EventBeginPlay
  (Components|Activation|Deactivate (Variables|Default|GetPressurePlateEffect)))

(event EventOnEndPressure
  (Rendering|Material|SetMaterial (Variables|Default|Getbody) 0 "/Game/Axelle/Props/Plaque_Pression_M.Plaque_Pression_M")
  (Rendering|Material|SetMaterial (Variables|Default|GetsecondBody) 0 "/Game/Axelle/Props/Plaque_Pression_M.Plaque_Pression_M"))

(event EventOnPressure
  (params (pressurePos :type Vector :default "0, 0, 0"))
  (bind _object (Variables|Default|Getobject))
  (bind _returnvalue (Transformation|GetActorLocation _object))
  (bind _returnvalue_2 (- _returnvalue pressurePos))
  (Utilities|FlowControl|Sequence
    (:then_0
      (Audio|PlaySoundatLocation "/Game/Sound/SD/PressurePlate/PressurePlateCue.PressurePlateCue" (Transformation|GetWorldLocation (Variables|Default|GetSpriteComponent)) "0, 0, 0" 1.0 1.0 0.0 0 0 0 0))
    (:then_1
      (Rendering|Material|SetMaterial (Variables|Default|Getbody) 0 "/Game/Axelle/Props/Plaque_Pression_Activated_M.Plaque_Pression_Activated_M")
      (Rendering|Material|SetMaterial (Variables|Default|GetsecondBody) 0 "/Game/Axelle/Props/Plaque_Pression_Activated_M.Plaque_Pression_Activated_M"))
    (:then_2
      (goto _label Stop))
    (:then_3
      (Transformation|SetRelativeLocation (Variables|Default|GetPressurePlateEffect) "0, 0, 0" false false)
      (Components|Activation|Activate (Variables|Default|GetPressurePlateEffect) true)
      (Components|MoveComponentTo (Variables|Default|GetPressurePlateEffect) (Math|Vector|MakeVector (.x _returnvalue_2) (.y _returnvalue_2) 0.0) "0, 0, 0" false false 2.0 false :!label _label)
      (Components|Activation|Deactivate (Variables|Default|GetPressurePlateEffect)))))

(fn ConstructionScript)