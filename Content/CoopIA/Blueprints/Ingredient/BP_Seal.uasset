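; BP_Seal is a seal actor that plays start, looping and end Niagara effects over its lifetime.
; BeginPlay either starts the seal or deactivates the effect, and sets collision from ActivateAtStart.
; StartSeal plays the start effect, then swaps to the during effect after a delay.
; EndSeal plays the end effect, then destroys the actor after a delay.
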(event Custom|Start%20Seal
  (Class|NiagaraComponent|SetAsset (Variables|Default|GetNiagara) "/Game/Axelle/FX/NS_Sceau_Start.NS_Sceau_Start" true)
  (Components|Activation|Activate (Variables|Default|GetNiagara) true)
  (Utilities|FlowControl|Delay 2.0)
  (Class|NiagaraComponent|SetAsset (Variables|Default|GetNiagara) "/Game/Axelle/FX/NS_Sceau_During.NS_Sceau_During" true)
  (Components|Activation|Activate (Variables|Default|GetNiagara) true))

(event Custom|End%20Seal
  (Class|NiagaraComponent|SetAsset (Variables|Default|GetNiagara) "/Game/Axelle/FX/NS_Sceau_End.NS_Sceau_End" true)
  (Components|Activation|Activate (Variables|Default|GetNiagara) true)
  (Utilities|FlowControl|Delay 2.0)
  (Actor|DestroyActor))

(event EventBeginPlay
  (if (Variables|Default|GetActivateAtStart)
    (CallFunction|StartSeal)
    (else
      (Components|Activation|Deactivate (Variables|Default|GetNiagara))))
  (Collision|SetActorEnableCollision (Variables|Default|GetActivateAtStart)))

(fn ConstructionScript)