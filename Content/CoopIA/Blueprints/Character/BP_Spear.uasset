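; BP_Spear is a character Blueprint for a spear form, themed as a kunai, that handles its feedback and external pushes.
; Entering the spear, charging a dash and dashing each play a sound cue, and dashing also spawns a kunai trail effect.
; Bullet hits launch the character with velocity override, while wind adds a small scaled launch.
; An event passes a texture to its player-count widget.
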(event EventWind
  (params (windDirection :type Vector :default "0, 0, 0"))
  (Character|LaunchCharacter (* windDirection 0.01) false false))

(event EventTick
  (params (DeltaSeconds :type Float%20%28single-precision%29)))

(event EventOnEnterSpear
  ;[1 1 1] SD
  (Audio|PlaySound2D "/Game/Sound/SD/Formations/Kunai/KunaiFormationCue.KunaiFormationCue" 1.0 1.0 0.0 0 0))

(event EventOnDash
  (bind _vfx (Variables|Default|GetVFX))
  (bind _returnvalue (Transformation|GetWorldTransform _vfx))
  ;[1 1 1] SD
  (Utilities|FlowControl|Sequence
    (:then_0
      (Audio|PlaySoundatLocation "/Game/Sound/SD/Formations/Kunai/KunaiDashCue.KunaiDashCue" (Transformation|GetActorLocation) "0, 0, 0" 1.0 1.0 0.0 0 0 0 0))
    (:then_1
      (bind _returnvalue_2 (Niagara|SpawnSystematLocation "/Game/Axelle/FX/NS_Trail_Kunai.NS_Trail_Kunai" (.location _returnvalue) (.rotation _returnvalue) "10.000000,10.000000,10.000000"))
      (Niagara|SpawnSystemAttached 0 _returnvalue_2 "None" "0, 0, 0" "0, 0, 0" "KeepRelativeOffset" false))))

(event EventOnDashLoad
  ;[1 1 1] SD
  (Utilities|FlowControl|Sequence
    (:then_0
      (Audio|PlaySoundatLocation "/Game/Sound/SD/Formations/Kunai/KunaiDashLoadCue.KunaiDashLoadCue" (Transformation|GetActorLocation) "0, 0, 0" 1.0 1.0 0.0 0 0 0 0))))

(event EventBulletHit
  (params (bulletDirection :type Vector :default "0, 0, 0"))
  (Character|LaunchCharacter (* bulletDirection (Variables|Default|GetBulletHitMultiplier)) true true))

(event EventUpdatePlayerCountUI
  (params (Texture :type Texture%202D%20Object%20Reference))
  ;[1 1 1] PlayerUI
  (bind _aswbp_player_count (Utilities|Casting|CastToWBP_PlayerCount (UserInterface|GetWidget (Variables|Default|GetWidget))))
  (Default|Init _aswbp_player_count Texture))

(fn ConstructionScript)