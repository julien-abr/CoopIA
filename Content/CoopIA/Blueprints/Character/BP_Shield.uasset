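; BP_Shield is a shield whose wall pivots around its WallOffset component in 45-degree yaw steps, driven by left and right rotation events.
; Each start event steps immediately, then repeats on a looping timer at the TurtleTimer interval until its completed event clears it.
; Both directions share a Multiplier clamped between -1 and 1, so opposing inputs cancel out.
; Interact is an empty placeholder marked for a sound.
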(event Custom|CustomEvent_1
  (Transformation|AddLocalRotation (Variables|Default|GetWallOffset) (Math|Rotator|MakeRotator 0.0 0.0 (Math|Conversions|ToFloat(Integer) (* (Variables|Default|GetMultiplier) 45))) false false))

(event Custom|CustomEvent
  (Transformation|AddLocalRotation (Variables|Default|GetWallOffset) (Math|Rotator|MakeRotator 0.0 0.0 (Math|Conversions|ToFloat(Integer) (* (Variables|Default|GetMultiplier) 45))) false false))

(event EventInteract)

(event EventRotationLeftStarted
  (Math|Integer|DecrementInt (Variables|Default|GetMultiplier)
    (:%20%20
      (Variables|Default|SetMultiplier (Math|Integer|Clamp(Integer) (Variables|Default|GetMultiplier) -1 1))
      (Transformation|AddLocalRotation (Variables|Default|GetWallOffset) (Math|Rotator|MakeRotator 0.0 0.0 (Math|Conversions|ToFloat(Integer) (* (Variables|Default|GetMultiplier) 45))) false false)
      (bind _returnvalue (Utilities|Time|SetTimerbyEvent (delegate Custom|CustomEvent) (Variables|Default|GetTurtleTimer) true))
      (Variables|Default|SetTimerLeft _returnvalue))))

(event EventRotationLeftCompleted
  (bind _timerleft (Variables|Default|GetTimerLeft))
  (Math|Integer|IncrementInt (Variables|Default|GetMultiplier)
    (:%20%20
      (Variables|Default|SetMultiplier (Math|Integer|Clamp(Integer) (Variables|Default|GetMultiplier) -1 1))
      (if (Utilities|Time|IsTimerActivebyHandle _timerleft)
        (Utilities|Time|ClearandInvalidateTimerbyHandle _timerleft)))))

(event EventRotationRightStarted
  (Math|Integer|IncrementInt (Variables|Default|GetMultiplier)
    (:%20%20
      (Variables|Default|SetMultiplier (Math|Integer|Clamp(Integer) (Variables|Default|GetMultiplier) -1 1))
      (Transformation|AddLocalRotation (Variables|Default|GetWallOffset) (Math|Rotator|MakeRotator 0.0 0.0 (Math|Conversions|ToFloat(Integer) (* (Variables|Default|GetMultiplier) 45))) false false)
      (bind _returnvalue (Utilities|Time|SetTimerbyEvent (delegate Custom|CustomEvent_1) (Variables|Default|GetTurtleTimer) true))
      (Variables|Default|SetTimerRight _returnvalue))))

(event EventRotationRightCompleted
  (bind _timerright (Variables|Default|GetTimerRight))
  (Math|Integer|DecrementInt (Variables|Default|GetMultiplier)
    (:%20%20
      (Variables|Default|SetMultiplier (Math|Integer|Clamp(Integer) (Variables|Default|GetMultiplier) -1 1))
      (if (Utilities|Time|IsTimerActivebyHandle _timerright)
        (Utilities|Time|ClearandInvalidateTimerbyHandle _timerright)))))

(fn ConstructionScript)