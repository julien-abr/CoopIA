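; Spirit AI character that plays pickup, idle and death sounds, with blue or red fox Niagara effects by index.
; It wraps AI Move To for points and actors, since task delegates can't be linked, swapping collision channel during actor transitions.
; A looping timer scales walk speed by distance to destination, at maximum during transitions.
; Hits from differently indexed characters launch it with a randomized cooldown; wind and bullets also push it.
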(event Custom|StartTimer
  (Utilities|Time|SetTimerbyEvent (delegate Custom|SetCanBeHit) (Math|Random|RandomFloatinRange 0.5 1.0)))

(event Custom|SetCanBeHit
  (Variables|Default|SetbCanBeHit true))

(event Custom|UpdateSpeed
  (if (Variables|Default|GetbTransition)
    (Variables|/Script/Engine.CharacterMovementComponent|SetMaxWalkSpeed (Variables|Character|GetCharacterMovement) (Variables|Default|GetMaxWalkSpeed))
    (else
      (Variables|/Script/Engine.CharacterMovementComponent|SetMaxWalkSpeed (Variables|Character|GetCharacterMovement) (Math|Float|Lerp (Variables|Default|GetMinWalkSpeed) (Variables|Default|GetMaxWalkSpeed) (/ (Math|Float|Clamp(Float) (Math|Vector|Distance(Vector) (Variables|Default|GetDestination) (Transformation|GetActorLocation)) 0.0 5e+02) 5e+02))))))

(event EventMove
  (params (Destination :type Vector :default "0, 0, 0") (AcceptanceRadius :type Float%20%28single-precision%29))
  ;[1 1 1] AI Move To (Blueprint because cant link delegate to Task result)
  (Variables|Default|SetDestination Destination)
  (AI|AIMoveTo self Destination 0 AcceptanceRadius false
    (:then
      (Class|CharacterBaseIA|Show))))

(event Collision|EventHit
  (params (MyComp :type Primitive%20Component%20Object%20Reference) (Other :type Actor%20Object%20Reference) (OtherComp :type Primitive%20Component%20Object%20Reference) (bSelfMoved :type Boolean) (HitLocation :type Vector :default "0, 0, 0") (HitNormal :type Vector :default "0, 0, 0") (NormalImpulse :type Vector :default "0, 0, 0") (Hit :type Hit%20Result%20Structure%20%28by%20ref%29))
  (bind _returnvalue (* HitNormal 1e+03))
  (bind _returnvalue_2 (* _returnvalue 4.0))
  (bind _ascharacter_base_ia (Utilities|Casting|CastToCharacterBaseIA Other))
  (if (Variables|Default|GetbCanBeHit)
    (if (not (== (Variables|/Script/CoopIA.CharacterBaseIA|GetPlayerIndex _ascharacter_base_ia) (Variables|Default|GetPlayerIndex)))
      (Class|NavMovementComponent|StopActiveMovement (Variables|Character|GetCharacterMovement))
      (Character|LaunchCharacter self (Math|Vector|MakeVector (.x _returnvalue_2) (.y _returnvalue_2) 0.0) false false)
      (Variables|Default|SetbCanBeHit false)
      (CallFunction|StartTimer)
      (Development|PrintString (Utilities|GetDisplayName Other)))))

(event EventMovetoActor
  (params (Target :type Actor%20Object%20Reference) (AcceptanceRadius :type Float%20%28single-precision%29))
  (Variables|Default|SetbTransition true)
  (Collision|SetCollisionObjectType (Variables|Default|GetCapsuleComponent) "ECC_GameTraceChannel3")
  (AI|AIMoveTo self "0, 0, 0" Target AcceptanceRadius false
    (:OnSuccess
      (Class|CharacterBaseIA|Succeeded)
      (Collision|SetCollisionObjectType (Variables|Default|GetCapsuleComponent) "ECC_GameTraceChannel2")
      (Variables|Default|SetbTransition false))
    (:OnFail
      (Class|CharacterBaseIA|Failed Target))))

(event EventWind
  (params (windDirection :type Vector :default "0, 0, 0"))
  (Character|LaunchCharacter (* windDirection 0.01) false false))

(event EventBeginPlay
  (Utilities|Time|SetTimerbyEvent (delegate Custom|UpdateSpeed) 0.1 true))

(event EventBulletHit
  (params (bulletDirection :type Vector :default "0, 0, 0"))
  (Class|NavMovementComponent|StopActiveMovement (Variables|Character|GetCharacterMovement))
  (Character|LaunchCharacter (* bulletDirection (Variables|Default|GetBulletHitMultiplier)) true true))

(event EventOnSpiritNeutral
  ;[1 1 1] Events - SD / VFX
  (Audio|PlaySoundatLocation "/Game/Sound/SD/Spirits/Idle/SpiritIdleCue.SpiritIdleCue" (Transformation|GetActorLocation) "0, 0, 0" 1.0 1.0 0.0 0 0 0 0))

(event EventOnSpiritDeath
  (params (Index :type Integer) (deathPos :type Vector :default "0, 0, 0"))
  (bind _returnvalue (Math|Vector|MakeVector (.x deathPos) (.y deathPos) 1e+01))
  (Utilities|FlowControl|Sequence
    (:then_0
      (Audio|PlaySoundatLocation "/Game/Sound/SD/Spirits/LoseSpirit/LoseSpiritCue.LoseSpiritCue" _returnvalue "0, 0, 0" 1.0 1.0 0.0 0 0 0 0)
      (Audio|PlaySoundatLocation "/Game/Sound/SD/Spirits/fallingSpirit/FallingSpiritCue.FallingSpiritCue" _returnvalue "0, 0, 0" 1.0 1.0 0.0 0 0 0 0))
    (:then_1
      (if (== Index 0)
        (Niagara|SpawnSystematLocation "/Game/Axelle/FX/NS_Blue_Fox_Dead.NS_Blue_Fox_Dead" _returnvalue "0, 0, 0" "20.000000,20.000000,20.000000")
        (else
          (Niagara|SpawnSystematLocation "/Game/Axelle/FX/NS_Red_Fox_Dead.NS_Red_Fox_Dead" "0, 0, 0" "0, 0, 0" "20.000000,20.000000,20.000000"))))))

(event EventOnSpiritPickup
  (params (Index :type Integer))
  (bind _vfx (Variables|Default|GetVFX))
  (bind _vfx_2 (Variables|Default|GetVFX))
  (bind _returnvalue (Transformation|GetWorldTransform _vfx))
  (bind _returnvalue_2 (Transformation|GetWorldTransform _vfx_2))
  ;[1 1 1] Events - SD / VFX
  (Utilities|FlowControl|Sequence
    (:then_0
      (Audio|PlaySoundatLocation "/Game/Sound/SD/Spirits/PickedUp/SpiritPickedUpCue.SpiritPickedUpCue" (Transformation|GetActorLocation) "0, 0, 0" 1.0 1.0 0.0 0 0 0 0))
    (:then_1
      (if (== Index 0)
        (Niagara|SpawnSystematLocation "/Game/Axelle/FX/NS_Touching_Spirit_02.NS_Touching_Spirit_02" (.location _returnvalue) (.rotation _returnvalue) "6.000000,6.000000,6.000000")
        (else
          (Niagara|SpawnSystematLocation "/Game/Axelle/FX/NS_Touching_Spirit.NS_Touching_Spirit" (.location _returnvalue_2) (.rotation _returnvalue_2) "6.000000,6.000000,6.000000"))))))

(fn ConstructionScript
  (|CallParentFunction))

(fn FindRandomPointAround)