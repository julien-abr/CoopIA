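; AI character Blueprint that moves to a point or actor and gets knocked back by other BP_IA characters.
; It wraps AIMoveTo because task delegates could not be linked, reporting actor-move results through Succeeded and Failed.
; Actor moves swap collision channel and run at full speed until success; otherwise a timer scales speed by destination distance.
; Hits launch it harder when PlayerIndex differs, followed by a random cooldown.
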(event Custom|StartTimer
  (Utilities|Time|SetTimerbyEvent (delegate Custom|SetCanBeHit) (Math|Random|RandomFloatinRange 0.5 1.0)))

(event Custom|SetCanBeHit
  (Variables|Default|SetbCanBeHit true))

(event Custom|UpdateSpeed
  (if (Variables|Default|GetbTransition)
    (Variables|/Script/Engine.CharacterMovementComponent|SetMaxWalkSpeed (Variables|Character|GetCharacterMovement) (Variables|Default|GetMaxWalkSpeed))
    (else
      (Variables|/Script/Engine.CharacterMovementComponent|SetMaxWalkSpeed (Variables|Character|GetCharacterMovement) (Math|Float|Lerp (Variables|Default|GetMinWalkSpeed) (Variables|Default|GetMaxWalkSpeed) (/ (Math|Float|Clamp(Float) (Math|Vector|Distance(Vector) (Variables|Default|GetDestination) (Transformation|GetActorLocation)) 0.0 5e+02) 5e+02))))))

(event EventMove
  (params (Destination :type Vector :default "0, 0, 0") (AcceptanceRadius :type Float%20%28single-precision%29))
  ;[1 1 1] AI Move To (Blueprint because cant link delegate to Task result)
  (Variables|Default|SetDestination Destination)
  (AI|AIMoveTo self Destination 0 AcceptanceRadius false))

(event Collision|EventHit
  (params (MyComp :type Primitive%20Component%20Object%20Reference) (Other :type Actor%20Object%20Reference) (OtherComp :type Primitive%20Component%20Object%20Reference) (bSelfMoved :type Boolean) (HitLocation :type Vector :default "0, 0, 0") (HitNormal :type Vector :default "0, 0, 0") (NormalImpulse :type Vector :default "0, 0, 0") (Hit :type Hit%20Result%20Structure%20%28by%20ref%29))
  (bind _returnvalue (* HitNormal 1e+03))
  (bind _self self)
  (bind _asbp_ia (Utilities|Casting|CastToBP_IA Other))
  (if (Variables|Default|GetbCanBeHit)
    (if (== (Variables|/Script/CoopIA.CharacterBaseIA|GetPlayerIndex _asbp_ia) (Variables|Default|GetPlayerIndex))
      (Character|LaunchCharacter _self (* _returnvalue 1.0) false false)
      (else
        (Character|LaunchCharacter _self (* _returnvalue 4.0) false false)))
    (Variables|Default|SetbCanBeHit false)
    (CallFunction|StartTimer)))

(event EventMovetoActor
  (params (Target :type Actor%20Object%20Reference) (AcceptanceRadius :type Float%20%28single-precision%29))
  (Variables|Default|SetbTransition true)
  (Collision|SetCollisionObjectType (Variables|Default|GetCapsuleComponent) "ECC_GameTraceChannel3")
  (AI|AIMoveTo self "0, 0, 0" Target AcceptanceRadius false
    (:OnSuccess
      (Class|CharacterBaseIA|Succeeded)
      (Collision|SetCollisionObjectType (Variables|Default|GetCapsuleComponent) "ECC_GameTraceChannel2")
      (Variables|Default|SetbTransition false))
    (:OnFail
      (Class|CharacterBaseIA|Failed Target))))

(event EventBeginPlay
  (Utilities|Time|SetTimerbyEvent (delegate Custom|UpdateSpeed) 0.1 true))

(fn ConstructionScript
  (|CallParentFunction))

(fn FindRandomPointAround)