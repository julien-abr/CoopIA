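; BP_SoundListener is a co-op actor that serves as the audio listener and crossfades zone music.
; On BeginPlay it attaches the first player controller's listener to its Cube, then each Tick follows the two pawns' horizontal midpoint, or player 0 when solo.
; InitMusic starts the Puzzle and Runner tracks and selects one from GameStateBaseCoop's ZoneType.
; Tick polls that ZoneType and crossfades between the tracks when it changes.
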(event Custom|InitMusic
  (Utilities|FlowControl|Sequence ; Then 0 C'est l'init où on lance tout\nThen 1 La en fonction du state de départ, on lance la bonne musique
    (:then_0
      (Audio|Components|Audio|SetSound (Variables|Default|GetMusPuzzleCue) (Variables|Default|GetPuzzleMusic))
      (Audio|Components|Audio|SetSound (Variables|Default|GetMusRunnerCue) (Variables|Default|GetRunnerMusic))
      (Audio|Components|Audio|Play (Variables|Default|GetMusPuzzleCue) 0.0)
      (Audio|Components|Audio|Play (Variables|Default|GetMusRunnerCue) 0.0))
    (:then_1
      (bind _output_get (Variables|Default|SetZoneType (Variables|/Script/CoopIA.GameStateBaseCoop|GetZoneType (Variables|Default|GetAs%20Game%20State%20Base%20Coop))))
      (if (== _output_get 0) ; 0 = Puzzle\n1 = Runner
        (Audio|Components|Audio|FadeOut (Variables|Default|GetMusRunnerCue) 0.0 0.0 "Linear" :!class /Script/Engine.AudioComponent)
        (Audio|Components|Audio|FadeIn (Variables|Default|GetMusPuzzleCue) 0.0 1.0 0.0 "Linear" :!class /Script/Engine.AudioComponent)
        (else
          (Audio|Components|Audio|FadeOut (Variables|Default|GetMusPuzzleCue) 0.0 0.0 "Linear" :!class /Script/Engine.AudioComponent)
          (Audio|Components|Audio|FadeIn (Variables|Default|GetMusRunnerCue) 0.0 1.0 0.0 "Linear" :!class /Script/Engine.AudioComponent))))))

(event EventTick
  (params (DeltaSeconds :type Float%20%28single-precision%29))
  (bind _returnvalue (Game|Player|GetPlayerPawn 1))
  (bind _returnvalue_2 (Game|Player|GetPlayerPawn 0))
  (bind _returnvalue_3 (Transformation|GetActorLocation _returnvalue))
  (bind _returnvalue_4 (Transformation|GetActorLocation _returnvalue_2))
  (Utilities|FlowControl|Sequence
    (:then_0
      (Transformation|SetActorLocation (Math|Vector|SelectVector (+ (/ (Math|Vector|MakeVector (- (.x _returnvalue_4) (.x _returnvalue_3)) (- (.y _returnvalue_4) (.y _returnvalue_3)) 0.0) 2) (Transformation|GetActorLocation (Game|Player|GetPlayerPawn 1))) (Transformation|GetActorLocation (Game|Player|GetPlayerPawn 0)) (Variables|Default|GetisTwoPlayer)) false false))
    (:then_1
      (if (!= (Math|Conversions|ToInteger(Byte) (Variables|Default|GetZoneType)) (Variables|/Script/CoopIA.GameStateBaseCoop|GetZoneType (Variables|Default|GetAs%20Game%20State%20Base%20Coop)))
        (bind _output_get (Variables|Default|SetZoneType (Variables|/Script/CoopIA.GameStateBaseCoop|GetZoneType (Variables|Default|GetAs%20Game%20State%20Base%20Coop)))) ; Switch Music
        (if (== _output_get 0) ; 0 = Puzzle\n1 = Runner
          (Audio|Components|Audio|FadeOut (Variables|Default|GetMusRunnerCue) 3.0 0.0 "Linear" :!class /Script/Engine.AudioComponent)
          (Audio|Components|Audio|FadeIn (Variables|Default|GetMusPuzzleCue) 2.0 1.0 0.0 "Linear" :!class /Script/Engine.AudioComponent)
          (else
            (Audio|Components|Audio|FadeOut (Variables|Default|GetMusPuzzleCue) 3.0 0.0 "Linear" :!class /Script/Engine.AudioComponent)
            (Audio|Components|Audio|FadeIn (Variables|Default|GetMusRunnerCue) 2.0 1.0 0.0 "Linear" :!class /Script/Engine.AudioComponent)))))))

(event EventBeginPlay
  (Utilities|FlowControl|Sequence
    (:then_0
      (Class|PlayerController|SetAudioListenerOverride (Game|GetPlayerController 0) (Variables|Default|GetCube) "0, 0, 0" "0, 0, 0"))
    (:then_1
      (bind _asgame_state_base_coop (Utilities|Casting|CastToGameStateBaseCoop (Game|GetGameState)))
      (Variables|Default|SetAs%20Game%20State%20Base%20Coop _asgame_state_base_coop))))

(fn ConstructionScript)