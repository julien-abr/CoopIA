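; BP_AIManager coordinates a group of AI companions around the player and switches them into formations.
; It registers the player and AIs, and in MOVE state a looping timer sends each AI to random points near the player.
; Formation changes send all AIs in front of the player and count down their arrivals.
; When all finish, only Spear is implemented: it hides the player and possesses a spawned BP_Spear.
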(event Custom|AddIA
  (params (IA :type BP%20IA%20Object%20Reference))
  ;[1 1 1] Setup Players & IA
  (Utilities|Array|Add (Variables|Default|GetArrayCharacterAI) IA))

(event Custom|RANDOM_MOVE
  (bind _player_0 (Variables|Default|GetPlayer_0))
  (bind _returnvalue (Transformation|GetActorLocation _player_0))
  ;[1 1 1] Random Move around Player
  (if (Utilities|Enum|Equal(Enum) (Variables|Default|GetEIAState) "RANDOM_MOVE")
    (Variables|Default|GetPlayer_0
      (:then
        (for _array_element (Variables|Default|GetArrayCharacterAI)
          (Default|MOVE _array_element (Math|Vector|MakeVector (+ (.x _returnvalue) (Math|Random|RandomFloatinRange -2e+02 2e+02)) (+ (.y _returnvalue) (Math|Random|RandomFloatinRange -2e+02 2e+02)) (.z _returnvalue)))))
      (:else))))

(event Custom|AddPlayer
  (params (Player :type BP%20Character%20Base%20Object%20Reference))
  ;[1 1 1] Setup Players & IA
  (bind _output_get (Variables|Default|SetPlayer_0 Player))
  (bind _asbp_player_controller (Utilities|Casting|CastToBP_PlayerController (Pawn|GetController _output_get)))
  (Variables|Default|SetPlayerController_0 _asbp_player_controller))

(event Custom|TransitionToFormation
  (params (EIAState :type EIAState%20Enum :default "RANDOM_MOVE"))
  (bind _arraycharacterai (Variables|Default|GetArrayCharacterAI))
  (bind _output_get (Variables|Default|SetEIAState EIAState))
  (switch Utilities|FlowControl|Switch|SwitchonEIAState _output_get
    (:MOVE_TO
      _)
    (:BALL
      _)
    (:SHIELD
      _)
    (:SPEAR
      _))
  (Variables|Default|SetNumberIA (Utilities|Array|Length _arraycharacterai))
  (for _array_element _arraycharacterai
    (Default|Transition _array_element (+ (* (Transformation|GetActorForwardVector (Variables|Default|GetPlayer_0)) 2e+02) (Transformation|GetActorLocation (Variables|Default|GetPlayer_0))))))

(event Custom|IA_SucesssTransition
  (bind _numberia (Variables|Default|GetNumberIA))
  (Math|Integer|DecrementInt _numberia
    (:%20%20
      (Development|PrintString (Utilities|String|ToString(Integer) _numberia))
      (if (== _numberia 0)
        (CallFunction|StartFormation)))))

(event Custom|StartFormation
  (switch Utilities|FlowControl|Switch|SwitchonEIAState (Variables|Default|GetEIAState)
    (:SPEAR
      (CallFunction|Spear))))

(event EventBeginPlay
  ;[1 1 1] Random Move around Player
  (Utilities|Time|SetTimerbyEvent (delegate Custom|RANDOM_MOVE) 2.0 true))

(fn ConstructionScript)

(fn Spear
  (bind _player_0 (Variables|Default|GetPlayer_0))
  (Default|HidePlayer _player_0)
  (Pawn|UnPossess (Variables|Default|GetPlayerController_0))
  (bind _returnvalue (Game|SpawnActorfromClass "/Game/CoopIA/Blueprints/Character/BP_Spear.BP_Spear_C" (Transformation|GetActorTransform _player_0) "AdjustIfPossibleButAlwaysSpawn" "MultiplyWithRoot" 0 0))
  (Pawn|Possess (Variables|Default|GetPlayerController_0) _returnvalue))