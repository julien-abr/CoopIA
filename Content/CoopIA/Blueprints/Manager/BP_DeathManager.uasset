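; Death manager Blueprint that plays the audio and visual feedback when a spirit or player dies.
; OnSpiritDeath and OnPlayerDeath play lose and falling spirit cues at DeathPos with fixed height, with player death adding a falling cue.
; Both then spawn a scaled Niagara fox-death effect, blue for index zero and red otherwise.
; Only the blue effect receives the death location; the red spawn leaves Location unset.
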(event EventOnPlayerDeath
  (params (Index :type Integer) (deathPos :type Vector :default "0, 0, 0"))
  (bind _returnvalue (Math|Vector|MakeVector (.x deathPos) (.y deathPos) 1e+01))
  ;[1 1 1] SD
  (Utilities|FlowControl|Sequence
    (:then_0
      (Audio|PlaySoundatLocation "/Game/Sound/SD/Falling/FallingCue.FallingCue" _returnvalue "0, 0, 0" 1.0 1.0 0.0 0 0 0 0)
      (Audio|PlaySoundatLocation "/Game/Sound/SD/Spirits/LoseSpirit/LoseSpiritCue.LoseSpiritCue" _returnvalue "0, 0, 0" 1.0 1.0 0.0 0 0 0 0)
      (Audio|PlaySoundatLocation "/Game/Sound/SD/Spirits/fallingSpirit/FallingSpiritCue.FallingSpiritCue" _returnvalue "0, 0, 0" 1.0 1.0 0.0 0 0 0 0))
    (:then_1
      (if (== Index 0)
        (Niagara|SpawnSystematLocation "/Game/Axelle/FX/NS_Blue_Fox_Dead.NS_Blue_Fox_Dead" _returnvalue "0, 0, 0" "20.000000,20.000000,20.000000")
        (else
          (Niagara|SpawnSystematLocation "/Game/Axelle/FX/NS_Red_Fox_Dead.NS_Red_Fox_Dead" "0, 0, 0" "0, 0, 0" "20.000000,20.000000,20.000000"))))))

(event EventOnSpiritDeath
  (params (Index :type Integer) (deathPos :type Vector :default "0, 0, 0"))
  (bind _returnvalue (Math|Vector|MakeVector (.x deathPos) (.y deathPos) 1e+01))
  ;[1 1 1] SD
  (Utilities|FlowControl|Sequence
    (:then_0
      (Audio|PlaySoundatLocation "/Game/Sound/SD/Spirits/LoseSpirit/LoseSpiritCue.LoseSpiritCue" _returnvalue "0, 0, 0" 1.0 1.0 0.0 0 0 0 0)
      (Audio|PlaySoundatLocation "/Game/Sound/SD/Spirits/fallingSpirit/FallingSpiritCue.FallingSpiritCue" _returnvalue "0, 0, 0" 1.0 1.0 0.0 0 0 0 0))
    (:then_1
      (if (== Index 0)
        (Niagara|SpawnSystematLocation "/Game/Axelle/FX/NS_Blue_Fox_Dead.NS_Blue_Fox_Dead" _returnvalue "0, 0, 0" "20.000000,20.000000,20.000000")
        (else
          (Niagara|SpawnSystematLocation "/Game/Axelle/FX/NS_Red_Fox_Dead.NS_Red_Fox_Dead" "0, 0, 0" "0, 0, 0" "20.000000,20.000000,20.000000"))))))

(fn ConstructionScript)