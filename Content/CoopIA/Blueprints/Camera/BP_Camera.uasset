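; BP_Camera is a shared camera for multiple players that keeps a tracked group in frame.
; Players register through an AddPlayers event.
; Each tick it lerps its location toward the players' average position using MoveSpeed.
; It also sets the spring arm length to the largest pairwise player distance, clamped between minimum and maximum values, so the view zooms out as players spread apart.
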(event Custom|AddPlayers
  (params (BP_Player :type BP%20Third%20Person%20Character%20Object%20Reference))
  (Utilities|Array|Add (Variables|Default|GetBP_Players) BP_Player))

(event EventTick
  (params (DeltaSeconds :type Float%20%28single-precision%29))
  (CallFunction|CalculateCamMovement)
  (CallFunction|UpdateArmLength))

(fn ConstructionScript)

(fn CalculateCamMovement
  (Variables|Default|SetPreviousLoc (Transformation|GetActorLocation))
  (bind _returnvalue (Class|GameplayStatics|GetActorArrayAverageLocation (Variables|Default|GetBP_Players)))
  (Transformation|SetActorLocation (Math|Vector|Lerp(Vector) (Variables|Default|GetPreviousLoc) _returnvalue (Variables|Default|GetMoveSpeed)) false false))

(fn UpdateArmLength
  (bind _bp_players (Variables|Default|GetBP_Players))
  (for (_array_element _array_index) _bp_players
    (Variables|Default|SetCurrentPlayer _array_element)
    (for _index (range (+ _array_index 1) (- (Utilities|Array|Length _bp_players) 1))
      (Utilities|Array|Add (Variables|Default|GetDistance) (Transformation|GetDistanceTo (Variables|Default|GetCurrentPlayer) (Utilities|Array|Get(acopy) (Variables|Default|GetBP_Players) _index)))))
  (Variables|/Script/Engine.SpringArmComponent|SetTargetArmLength (Variables|Default|GetSpringArm) (Math|Float|Clamp(Float) (.MaxValue (Math|Float|MaxOfFloatArray (Variables|Default|GetDistance))) (Variables|Default|GetMinArmLength) (Variables|Default|GetMaxArmLength)))
  (Utilities|Array|Clear (Variables|Default|GetDistance)))