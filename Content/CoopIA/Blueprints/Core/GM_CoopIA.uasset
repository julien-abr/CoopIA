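; Co-op game mode with unused setup logic for local multiplayer on a shared camera; BeginPlay and the construction script are empty.
; The disconnected graph creates a local player per PlayerStart after a short delay, then spawns and possesses a character for each.
; Each character registers with BP_Camera, which becomes that controller's view target.
; Player one gets a separate branch that adds the Enhanced Input mapping context.
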(event EventBeginPlay)

(fn ConstructionScript)