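; Trigger volume that shows a tutorial sprite when a player walks into it.
; On box overlap it accepts either local player character (index 0 or 1) and passes its TutoSprite to MyGameInstance, setting the ShowTuto flag.
; The box collider then destroys itself, so each trigger fires only once.
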(event OnComponentBeginOverlap(Box_Collider)
  (params (OverlappedComponent :type Primitive%20Component%20Object%20Reference) (OtherActor :type Actor%20Object%20Reference) (OtherComp :type Primitive%20Component%20Object%20Reference) (OtherBodyIndex :type Integer) (bFromSweep :type Boolean) (SweepResult :type Hit%20Result%20Structure%20%28by%20ref%29))
  (bind _ascharacter_base (Utilities|Casting|CastToCharacterBase (Game|GetPlayerCharacter 0)))
  (if (== _ascharacter_base OtherActor)
    (bind _asmy_game_instance (Utilities|Casting|CastToMyGameInstance (Game|GetGameInstance) :!label _label))
    (Variables|/Game/Levels/Menus/Misc/MyGameInstance.MyGameInstance_C|SetTuto_to_display _asmy_game_instance (Variables|Default|GetTuto_Sprite))
    (Variables|/Game/Levels/Menus/Misc/MyGameInstance.MyGameInstance_C|SetShow_Tuto _asmy_game_instance true)
    (Components|DestroyComponent (Variables|Default|GetBox_Collider))
    (else
      (bind _ascharacter_base_2 (Utilities|Casting|CastToCharacterBase (Game|GetPlayerCharacter 1)))
      (if (== _ascharacter_base_2 OtherActor)
        (goto _label)))))

(fn ConstructionScript)