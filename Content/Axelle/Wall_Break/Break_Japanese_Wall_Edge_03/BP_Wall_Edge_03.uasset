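; Broken Japanese wall edge Blueprint that animates a material fade on its pieces as soon as play begins.
; BeginPlay creates a dynamic instance of the first material on each static mesh component and stores it in an array.
; Tick advances a timer and drives FadeAmount on every instance from -1 to 1 over two seconds.
; The timer is never clamped or stopped, so the value keeps rising afterward.
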(event EventBeginPlay
  (for _array_element (Actor|GetComponentsByClass "/Script/Engine.StaticMeshComponent")
    (bind _asstatic_mesh_component (Utilities|Casting|CastToStaticMeshComponent _array_element))
    (bind _returnvalue (Rendering|Material|CreateDynamicMaterialInstance _asstatic_mesh_component 0 (Rendering|Material|GetMaterial _asstatic_mesh_component 0) "None" :!class /Script/Engine.PrimitiveComponent))
    (Rendering|Material|SetMaterial _asstatic_mesh_component 0 _returnvalue)
    (Utilities|Array|Add (Variables|Default|GetDynamicMaterialArray) _returnvalue)))

(event EventTick
  (params (DeltaSeconds :type Float%20%28single-precision%29))
  (Variables|Default|Settimer (+ (/ DeltaSeconds 2.0) (Variables|Default|Gettimer)))
  (for _array_element (Variables|Default|GetDynamicMaterialArray)
    (Rendering|Material|SetScalarParameterValue _array_element "FadeAmount" (Math|Float|Lerp -1.0 1.0 (Variables|Default|Gettimer)) :!class /Script/Engine.MaterialInstanceDynamic)))

(event Collision|EventActorBeginOverlap
  (params (OtherActor :type Actor%20Object%20Reference)))

(fn ConstructionScript)