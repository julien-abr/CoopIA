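; BP_Hex is a builder-tool hex Blueprint whose mesh can be made to shake through StartShaking and StopShaking events.
; StartShaking randomly picks an amplitude multiplier and one of three timeline curves, so shakes vary.
; Each timeline update applies the scaled curve value equally to X, Y and Z of the mesh's relative location, with sweep.
; StopShaking halts the timeline without resetting the mesh position.
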(event EventStartShaking
  (Variables|Default|SetRandomMultiplier (Math|Random|RandomFloatinRange 2.0 1e+01))
  (Variables|Default|SetRandomTimeline (Math|Random|RandomIntegerinRange 0 2))
  (bind (_direction _shake _shake_2 _shake3) (Timeline|ShakingTimeline Play)
    (:Update
      (switch int (Variables|Default|GetRandomTimeline)
        (:0
          (Transformation|SetRelativeLocation (Variables|Default|Get_hexMesh) (Math|Vector|MakeVector (* _shake (Variables|Default|GetRandomMultiplier)) (* _shake (Variables|Default|GetRandomMultiplier)) (* _shake (Variables|Default|GetRandomMultiplier))) true false))
        (:1
          (Transformation|SetRelativeLocation (Variables|Default|Get_hexMesh) (Math|Vector|MakeVector (* _shake_2 (Variables|Default|GetRandomMultiplier)) (* _shake_2 (Variables|Default|GetRandomMultiplier)) (* _shake_2 (Variables|Default|GetRandomMultiplier))) true false))
        (:2
          (Transformation|SetRelativeLocation (Variables|Default|Get_hexMesh) (Math|Vector|MakeVector (* _shake3 (Variables|Default|GetRandomMultiplier)) (* _shake3 (Variables|Default|GetRandomMultiplier)) (* _shake3 (Variables|Default|GetRandomMultiplier))) true false))))))

(event EventStopShaking
  (bind (_direction _shake _shake_2 _shake3) (Timeline|ShakingTimeline Stop)
    (:Update
      (switch int (Variables|Default|GetRandomTimeline)
        (:0
          (Transformation|SetRelativeLocation (Variables|Default|Get_hexMesh) (Math|Vector|MakeVector (* _shake (Variables|Default|GetRandomMultiplier)) (* _shake (Variables|Default|GetRandomMultiplier)) (* _shake (Variables|Default|GetRandomMultiplier))) true false))
        (:1
          (Transformation|SetRelativeLocation (Variables|Default|Get_hexMesh) (Math|Vector|MakeVector (* _shake_2 (Variables|Default|GetRandomMultiplier)) (* _shake_2 (Variables|Default|GetRandomMultiplier)) (* _shake_2 (Variables|Default|GetRandomMultiplier))) true false))
        (:2
          (Transformation|SetRelativeLocation (Variables|Default|Get_hexMesh) (Math|Vector|MakeVector (* _shake3 (Variables|Default|GetRandomMultiplier)) (* _shake3 (Variables|Default|GetRandomMultiplier)) (* _shake3 (Variables|Default|GetRandomMultiplier))) true false))))))

(fn ConstructionScript)