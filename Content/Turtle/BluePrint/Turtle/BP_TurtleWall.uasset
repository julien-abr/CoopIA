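; Turtle formation wall actor that the player rotates, adding the IMC_Turtle input context on spawn and removing it when destroyed.
; Left and right inputs turn WallOffset in 45-degree steps, repeating on looping timers while held, with a shared Test counter setting direction.
; Turtle or neutral formation input destroys the wall; neutral also clears the character's IsTurtleOn.
; Older direction-snapping rotation logic remains disconnected, and Interact only prints a debug string.
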(event Custom|ResetTimer
  (bind _returnvalue (Class|KismetMathLibrary|VectorForward))
  (bind _returnvalue_2 (Math|Vector2D|Normalize2D))
  (bind _returnvalue_3 (Math|Conversions|ToVector2D(Vector) _returnvalue))
  (bind _returnvalue_4 (Math|Vector2D|DotProduct(2D) _returnvalue_2 _returnvalue_3))
  (bind _returnvalue_5 (Class|KismetMathLibrary|DegAcos _returnvalue_4))
  (bind _returnvalue_6 (/ _returnvalue_5 45.0))
  (bind _returnvalue_7 (Class|KismetMathLibrary|Round64 _returnvalue_6))
  (bind _returnvalue_8 (* _returnvalue_7 45))
  (bind _returnvalue_9 (Math|Conversions|ToFloat(Integer) _returnvalue_8))
  ;[0 0 0] OLD
  (Rendering|SetVisibility (Variables|Default|GetCube) true false)
  (if (> (.Y (Math|Vector2D|BreakVector2D)) 0.0)
    (Transformation|SetRelativeRotation (Variables|Default|GetWallOffset) (Math|Rotator|MakeRotator 0.0 0.0 _returnvalue_9) false false)
    (else
      (Transformation|SetRelativeRotation (Variables|Default|GetWallOffset) (Math|Rotator|MakeRotator 0.0 0.0 (* _returnvalue_9 -1.0)) false false)))
  (Variables|Default|SethasRotate true))

(event Custom|CustomEvent_1
  (Transformation|AddLocalRotation (Variables|Default|GetWallOffset) (Math|Rotator|MakeRotator 0.0 0.0 (Math|Conversions|ToFloat(Integer) (* (Variables|Default|Gettest) 45))) false false))

(event Custom|CustomEvent
  (Transformation|AddLocalRotation (Variables|Default|GetWallOffset) (Math|Rotator|MakeRotator 0.0 0.0 (Math|Conversions|ToFloat(Integer) (* (Variables|Default|Gettest) 45))) false false))

(event Input|EnhancedActionEvents|EnhancedInputActionIA_NeutralFormation
  (params (ActionValue :type Boolean) (ElapsedSeconds :type Float%20%28double-precision%29) (TriggeredSeconds :type Float%20%28double-precision%29) (InputAction :type Input%20Action%20Object%20Reference :default "/Game/Turtle/Input/InputAction/IA_NeutralFormation.IA_NeutralFormation"))
  (:Started
    (Variables|/Game/Turtle/BluePrint/BP_TurtleCharacter.BP_TurtleCharacter_C|SetisTurtleOn (Variables|Default|GetCharacter) false)
    (Actor|DestroyActor)))

(event Input|EnhancedActionEvents|EnhancedInputActionIA_TurtleFormation
  (params (ActionValue :type Boolean) (ElapsedSeconds :type Float%20%28double-precision%29) (TriggeredSeconds :type Float%20%28double-precision%29) (InputAction :type Input%20Action%20Object%20Reference :default "/Game/Turtle/Input/InputAction/IA_TurtleFormation.IA_TurtleFormation"))
  (:Started
    (Actor|DestroyActor)))

(event Input|EnhancedActionEvents|EnhancedInputActionIA_TurtleRotationLeft
  (params (ActionValue :type Boolean) (ElapsedSeconds :type Float%20%28double-precision%29) (TriggeredSeconds :type Float%20%28double-precision%29) (InputAction :type Input%20Action%20Object%20Reference :default "/Game/Turtle/Input/InputAction/IA_TurtleRotationLeft.IA_TurtleRotationLeft"))
  (:Started
    (Math|Integer|DecrementInt (Variables|Default|Gettest)
      (:%20%20
        (Transformation|AddLocalRotation (Variables|Default|GetWallOffset) (Math|Rotator|MakeRotator 0.0 0.0 (Math|Conversions|ToFloat(Integer) (* (Variables|Default|Gettest) 45))) false false)
        (bind _returnvalue (Utilities|Time|SetTimerbyEvent (delegate Custom|CustomEvent) (Variables|Default|GetTurtleTimer) true))
        (Variables|Default|SetTimerLeft _returnvalue))))
  (:Completed
    (Math|Integer|IncrementInt (Variables|Default|Gettest)
      (:%20%20
        (if (Utilities|Time|IsTimerActivebyHandle (Variables|Default|GetTimerLeft))
          (Utilities|Time|ClearandInvalidateTimerbyHandle (Variables|Default|GetTimerLeft)))))))

(event Input|EnhancedActionEvents|EnhancedInputActionIA_TurtleRotationRight
  (params (ActionValue :type Boolean) (ElapsedSeconds :type Float%20%28double-precision%29) (TriggeredSeconds :type Float%20%28double-precision%29) (InputAction :type Input%20Action%20Object%20Reference :default "/Game/Turtle/Input/InputAction/IA_TurtleRotationRight.IA_TurtleRotationRight"))
  (:Started
    (Math|Integer|IncrementInt (Variables|Default|Gettest)
      (:%20%20
        (Transformation|AddLocalRotation (Variables|Default|GetWallOffset) (Math|Rotator|MakeRotator 0.0 0.0 (Math|Conversions|ToFloat(Integer) (* (Variables|Default|Gettest) 45))) false false)
        (bind _returnvalue (Utilities|Time|SetTimerbyEvent (delegate Custom|CustomEvent_1) (Variables|Default|GetTurtleTimer) true))
        (Variables|Default|SetTimerRight _returnvalue))))
  (:Completed
    (Math|Integer|DecrementInt (Variables|Default|Gettest)
      (:%20%20
        (if (Utilities|Time|IsTimerActivebyHandle (Variables|Default|GetTimerRight))
          (Utilities|Time|ClearandInvalidateTimerbyHandle (Variables|Default|GetTimerRight)))))))

(event EventInteract
  (Development|PrintString "Hello"))

(event EventBeginPlay
  (bind _returnvalue (Game|GetPlayerController 0))
  (bind _returnvalue_2 (PlayerController|LocalPlayerSubsystems|GetEnhancedInputLocalPlayerSubsystem _returnvalue))
  (Utilities|IsValid _returnvalue_2
    (:Is%20Valid
      (Input|AddMappingContext _returnvalue_2 "/Game/Turtle/Input/IMC_Turtle.IMC_Turtle" 1 "(bIgnoreAllPressedKeysUntilRelease=True,bForceImmediately=False,bNotifyUserSettings=False)")
      (Input|EnableInput _returnvalue))))

(event EventDestroyed
  (bind _returnvalue (Game|GetPlayerController 0))
  (bind _returnvalue_2 (PlayerController|LocalPlayerSubsystems|GetEnhancedInputLocalPlayerSubsystem _returnvalue))
  (Utilities|IsValid _returnvalue_2
    (:Is%20Valid
      (Input|RemoveMappingContext _returnvalue_2 "/Game/Turtle/Input/IMC_Turtle.IMC_Turtle" "(bIgnoreAllPressedKeysUntilRelease=True,bForceImmediately=False,bNotifyUserSettings=False)"))))

(fn ConstructionScript)